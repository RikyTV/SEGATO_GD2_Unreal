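; Combat component for BP_ThirdPersonCharacter that handles target lock and sword combo attacks.
; Lock input toggles a camera-forward pawn sphere trace, attaches a marker actor to the hit, and switches movement to controller rotation, which Tick aims at the target.
; Attack input plays a combo montage; further presses buffer continuation, otherwise a notify stops it.
; A looping damage-trace timer is stubbed, with trace results unused.
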(event Custom|Begin%20Damage%20Trace
  (Utilities|Time|SetTimerbyEvent (delegate Custom|Damage%20Trace) 0.01 true))

(event Custom|Damage%20Trace
  (Collision|MultiSphereTraceByChannel "0, 0, 0" "0, 0, 0" 0.0 "TraceTypeQuery1" false 0 "None"))

(event Input|EnhancedActionEvents|EnhancedInputActionIA_Lock
  (params (ActionValue :type Boolean) (ElapsedSeconds :type Float%20%28double-precision%29) (TriggeredSeconds :type Float%20%28double-precision%29) (InputAction :type Input%20Action%20Object%20Reference :default "/Game/ThirdPerson/Input/Actions/IA_Lock.IA_Lock"))
  (bind _returnvalue (Game|GetPlayerCameraManager 0))
  (bind _player_bp (Variables|Default|GetPlayer%20BP))
  (bind _player_bp_2 (Variables|Default|GetPlayer%20BP))
  (bind _transformcomponent (Variables|/Script/Engine.PlayerCameraManager|GetTransformComponent _returnvalue))
  (bind _charactermovement (Variables|/Script/Engine.Character|GetCharacterMovement _player_bp_2))
  (bind _charactermovement_2 (Variables|/Script/Engine.Character|GetCharacterMovement _player_bp))
  (bind _returnvalue_2 (Transformation|GetWorldLocation _transformcomponent))
  (bind _returnvalue_3 (+ (.z _returnvalue_2) 1.5e+02))
  (bind _returnvalue_4 (Math|Vector|MakeVector (.x _returnvalue_2) (.y _returnvalue_2) _returnvalue_3))
  ;[0.15 0.15 0.15 0.5] Target Lock
  (:Started
    (Variables|Default|GetTarget%20Lock%20Actor
      (:then
        (Variables|Default|SetTarget%20Lock%20Actor 0)
        (Variables|/Script/Engine.CharacterMovementComponent|SetbOrientRotationToMovement _charactermovement true)
        (Variables|/Script/Engine.CharacterMovementComponent|SetbUseControllerDesiredRotation _charactermovement false)
        (Actor|DestroyActor (Variables|Default|GetTarget%20Lock%20Widget)))
      (:else
        (bind (_outhit _returnvalue_5) (Collision|SphereTraceForObjects _returnvalue_4 (+ _returnvalue_4 (* (Math|Vector|GetForwardVector (Transformation|GetWorldRotation _transformcomponent)) (Variables|Default|GetMaxDistance))) (Variables|Default|GetMaxRadius) (Utilities|Array|MakeArray "ObjectTypeQuery3") false 0 "ForDuration" true "(R=1.000000,G=0.000000,B=0.000000,A=1.000000)" "(R=0.000000,G=1.000000,B=0.000000,A=1.000000)" 2.0))
        (if _returnvalue_5
          (Variables|Default|SetTarget%20Lock%20Actor (.HitActor (Collision|BreakHitResult _outhit)))
          (Variables|/Script/Engine.CharacterMovementComponent|SetbOrientRotationToMovement _charactermovement_2 false)
          (Variables|/Script/Engine.CharacterMovementComponent|SetbUseControllerDesiredRotation _charactermovement_2 true)
          (bind _returnvalue_6 (Game|SpawnActorfromClass "/Game/Blueprints/BP_TargetLockWidget.BP_TargetLockWidget_C" (Math|Transform|MakeTransform "0, 0, 0" "0, 0, 0" "1.000000,1.000000,1.000000") "AlwaysSpawn" "MultiplyWithRoot" 0 0))
          (bind _output_get (Variables|Default|SetTarget%20Lock%20Widget _returnvalue_6))
          (Transformation|AttachActorToActor _output_get (Variables|Default|GetTarget%20Lock%20Actor) "None" "SnapToTarget" "KeepRelative" "KeepRelative" true))))))

(event Input|EnhancedActionEvents|EnhancedInputActionIA_Attack
  (params (ActionValue :type Boolean) (ElapsedSeconds :type Float%20%28double-precision%29) (TriggeredSeconds :type Float%20%28double-precision%29) (InputAction :type Input%20Action%20Object%20Reference :default "/Game/ThirdPerson/Input/Actions/IA_Attack.IA_Attack"))
  ;[0.15 0.15 0.15 0.5] Sword Combo Animation
  (:Started
    (if (not (Variables|Default|GetisAttacking))
      (Variables|Default|SetisAttacking true)
      (Animation|Montage|PlayMontage (Variables|/Script/Engine.Character|GetMesh (Variables|Default|GetPlayer%20BP)) "/Game/Characters/Souls/Combat/SwordAttackCombo_Montage.SwordAttackCombo_Montage"
        (:OnCompleted
          (Variables|Default|SetisAttacking false :!label _label))
        (:OnInterrupted
          (goto _label))
        (:OnNotifyBegin
          (if (and (Variables|Default|GetisAttacking) (Variables|Default|Getcombo))
            (Variables|Default|Setcombo false)
            (else
              (Animation|Montage|MontageStop (Components|SkeletalMesh|GetAnimInstance (Variables|/Script/Engine.Character|GetMesh (Variables|Default|GetPlayer%20BP))) 0.2 "/Game/Characters/Souls/Combat/SwordAttackCombo_Montage.SwordAttackCombo_Montage")))))
      (else
        (Variables|Default|Setcombo true)))))

(event EventTick
  (params (DeltaSeconds :type Float%20%28single-precision%29))
  (bind _player_bp (Variables|Default|GetPlayer%20BP))
  (bind _target_lock_actor (Variables|Default|GetTarget%20Lock%20Actor))
  (bind _returnvalue (Transformation|GetActorLocation _target_lock_actor))
  (bind _returnvalue_2 (Transformation|GetActorLocation _player_bp))
  (bind _returnvalue_3 (Math|Rotator|FindLookatRotation _returnvalue_2 _returnvalue))
  ;[0.15 0.15 0.15 0.5] Target Lock
  ;;[0.15 0.15 0.15 0.5] Target Lock Update
  (Variables|Default|GetTarget%20Lock%20Actor
    (:then
      (Pawn|SetControlRotation (Pawn|GetController _player_bp) (Math|Rotator|MakeRotator (.roll _returnvalue_3) (+ (.pitch _returnvalue_3) -25.0) (.yaw _returnvalue_3))))
    (:else)))

(event EventBeginPlay
  ;[0.15 0.15 0.15 0.5] Get Player Class
  (bind _asbp_third_person_character (Utilities|Casting|CastToBP_ThirdPersonCharacter (Components|GetOwner)))
  (Variables|Default|SetPlayer%20BP _asbp_third_person_character))